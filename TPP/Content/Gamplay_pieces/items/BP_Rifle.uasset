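; BP_Rifle is an interactable rifle pickup that destroys itself when used.
; On interact, it casts to the player's BP_ThirdPersonCharacter and adds that character's ItemList into its own RifleItem set, leaving the character's list unchanged.
; It caches the character on BeginPlay and, on a name request, sets that character's UI name to "Axe" despite being the rifle.
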(event `/Game/interfaces/BPI_Interact.OnInteract`
  (bind _asbp_third_person_character (cast `/Game/ThirdPerson/Blueprints/BP_ThirdPersonCharacter` (`GameplayStatics.GetPlayerCharacter` 0)))
  (`BlueprintSetLibrary.Set_AddItems` (`self.RifleItem`) (`/Game/ThirdPerson/Blueprints/BP_ThirdPersonCharacter.ItemList` _asbp_third_person_character))
  (`self.K2_DestroyActor`))

(event `/Game/interfaces/BPI_GetThing.OnGetName`
  (params (ItemNamed :type String))
  (set `/Game/ThirdPerson/Blueprints/BP_ThirdPersonCharacter.NameForUI` "Axe" (`self.CHAR`)))

(event `self.ReceiveBeginPlay`
  (bind _returnvalue (`GameplayStatics.GetActorOfClass` "/Game/ThirdPerson/Blueprints/BP_ThirdPersonCharacter.BP_ThirdPersonCharacter_C"))
  (set `self.CHAR` _returnvalue))

(fn `UserConstructionScript`)