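; BP_HealthPickup is a MedKit pickup that heals the third-person player character on interaction.
; OnInteract adds a fixed amount to the character's HealthVal, clamps it within the health range and destroys the pickup.
; On BeginPlay it caches the character by class lookup, and OnGetName writes the item's display name into that character's NameForUI variable.
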(event `/Game/interfaces/BPI_Interact.OnInteract`
  (bind _asbp_third_person_character (cast `/Game/ThirdPerson/Blueprints/BP_ThirdPersonCharacter` (`GameplayStatics.GetPlayerCharacter` 0)))
  (set `/Game/ThirdPerson/Blueprints/BP_ThirdPersonCharacter.healthVal` (`KismetMathLibrary.FClamp` (+ (`/Game/ThirdPerson/Blueprints/BP_ThirdPersonCharacter.healthVal` _asbp_third_person_character) 50.0) 0.0 100.0) _asbp_third_person_character)
  (`self.K2_DestroyActor`))

(event `/Game/interfaces/BPI_GetThing.OnGetName`
  (params (ItemNamed :type String))
  (set `/Game/ThirdPerson/Blueprints/BP_ThirdPersonCharacter.NameForUI` "MedKit" (`self.Char`)))

(event `self.ReceiveBeginPlay`
  (bind _returnvalue (`GameplayStatics.GetActorOfClass` "/Game/ThirdPerson/Blueprints/BP_ThirdPersonCharacter.BP_ThirdPersonCharacter_C"))
  (set `self.Char` _returnvalue))

(fn `UserConstructionScript`)