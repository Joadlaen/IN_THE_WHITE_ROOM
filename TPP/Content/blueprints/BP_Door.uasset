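; BP_Door is a bunker door actor that swings open on interaction when the player character holds a key.
; On BeginPlay it caches the BP_ThirdPersonCharacter found in the level and later reads its HasKey flag in OnInteract.
; The door mesh snaps to an absolute 90-degree world yaw without interpolation.
; The branch that would set it back to closed has a constant true condition, so it never runs.
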(event `self.ReceiveBeginPlay`
  (bind _returnvalue (`GameplayStatics.GetActorOfClass` "/Game/ThirdPerson/Blueprints/BP_ThirdPersonCharacter.BP_ThirdPersonCharacter_C"))
  (set `self.CharREF` _returnvalue))

(event `/Game/interfaces/BPI_Interact.OnInteract`
  (if (`/Game/ThirdPerson/Blueprints/BP_ThirdPersonCharacter.HasKey` (`self.CharREF`))
    (if true
      (set `self.DoorYaw` 90.0)
      (else
        (set `self.DoorYaw` 0.0)))
    (`SceneComponent.K2_SetWorldRotation` (`self.SM_Bunker_Door`) (`KismetMathLibrary.MakeRotator` 0.0 0.0 (`self.DoorYaw`)) false false)))

(fn `UserConstructionScript`)