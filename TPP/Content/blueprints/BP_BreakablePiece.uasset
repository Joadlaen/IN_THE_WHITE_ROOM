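; BP_BreakablePiece is a breakable block that is destroyed when damaged while the player has the axe equipped.
; BeginPlay caches the BP_ThirdPersonCharacter, whose AxeEquipped flag gates destruction in OnDamage.
; OnGetName writes the block's display name to that character's NameForUI variable.
; The Construction Script applies the NewMesh variable to the static mesh, so the block's look can vary per instance.
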(event `self.ReceiveBeginPlay`
  (bind _returnvalue (`GameplayStatics.GetActorOfClass` "/Game/ThirdPerson/Blueprints/BP_ThirdPersonCharacter.BP_ThirdPersonCharacter_C"))
  (set `self.CharREF` _returnvalue))

(event `/Game/interfaces/BPI_Damage.OnDamage`
  (if (`/Game/ThirdPerson/Blueprints/BP_ThirdPersonCharacter.AxeEquipped` (`self.CharREF`))
    (`self.K2_DestroyActor`)))

(event `/Game/interfaces/BPI_GetThing.OnGetName`
  (params (ItemNamed :type String))
  (set `/Game/ThirdPerson/Blueprints/BP_ThirdPersonCharacter.NameForUI` "Breakable block" (`self.CharREF`)))

(fn `UserConstructionScript`
  (`StaticMeshComponent.SetStaticMesh` (`self.StaticMesh`) (`self.New Mesh`)))