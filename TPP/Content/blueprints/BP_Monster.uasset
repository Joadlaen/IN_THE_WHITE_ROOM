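; BP_Monster is a monster that pursues the player and sends a damage message to any actor entering its DeathBox.
; MonsantoEyes perception updates order its pawn to the player's location, whether the stimulus was gained or lost.
; While the last stimulus is not a successful sense, Tick repeatedly requests moves to random navigable points tightly around the player, with no pawn specified.
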(event `self.ReceiveTick`
  (params (DeltaSeconds :type "Float (single-precision)"))
  (if (not (`.bSuccessfullySensed` (break `AIStimulus` (stale `self.MonsantoEyes.OnTargetPerceptionUpdated` Stimulus))))
    (bind _randomlocation (`NavigationSystemV1.K2_GetRandomLocationInNavigableRadius` (`self.K2_GetActorLocation` (`GameplayStatics.GetPlayerCharacter` 0)) 10.0 null null))
    (`|AIMoveTo` null _randomlocation null)))

(event `self.MonsantoEyes.OnTargetPerceptionUpdated`
  (params (Actor :type "Actor Object Reference") (Stimulus :type "AIStimulus Structure"))
  (`|AIMoveTo` (`PawnMovementComponent.GetPawnOwner` (`self.Monsanto move`)) (`self.K2_GetActorLocation` (`GameplayStatics.GetPlayerCharacter` 0)) null))

(event `self.DeathBox.OnComponentBeginOverlap`
  (params (OverlappedComponent :type "PrimitiveComponent Object Reference") (OtherActor :type "Actor Object Reference") (OtherComp :type "PrimitiveComponent Object Reference") (OtherBodyIndex :type Integer) (bFromSweep :type Boolean) (SweepResult :type "HitResult Structure (by ref)"))
  (message `/Game/interfaces/BPI_Damage.OnDamage` OtherActor))

(fn `UserConstructionScript`)